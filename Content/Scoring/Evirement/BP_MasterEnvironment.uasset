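; Master destructible environment actor that has HP and pays out points and style points to the player who damages it.
; Incoming damage is capped at remaining HP and converted to a percentage of max HP, which sets the share of both rewards sent to the instigator's PlayerState.
; The actor drains its own style pool alongside HP, shows both on a WBP_ActorStats widget, and destroys itself at zero HP.
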(event `self.ReceiveBeginPlay`
  (bind _aswbp_actor_stats (cast `/Game/Scoring/Evirement/UI/WBP_ActorStats` (`WidgetComponent.GetWidget` (`self.Widget`))))
  (set `self.As WBP Actor Stats` _aswbp_actor_stats)
  (`/Game/Scoring/Evirement/UI/WBP_ActorStats.SetTextValues` (`self.As WBP Actor Stats`) (`self.CurrentHP`) (`self.MaxHP`) (`self.CurrentStylePoints`) (`self.StylePoints`)))

(event `self.ReceiveAnyDamage`
  (params (Damage :type "Float (single-precision)") (DamageType :type "DamageType Object Reference") (InstigatedBy :type "Controller Object Reference") (DamageCauser :type "Actor Object Reference"))
  (bind _returnvalue (* (/ (`self.StylePoints`) 100.0) (`self.ReceivedDamagePercent`)))
  (`self.ReceiveDamage` Damage)
  (message `/Game/Scoring/BPI_PlayerState.IncreasePoints` (`Controller.PlayerState` InstigatedBy) (* (/ (`self.Points`) 100.0) (`self.ReceivedDamagePercent`)) _returnvalue)
  (set `self.CurrentStylePoints` (- (`self.CurrentStylePoints`) _returnvalue))
  (`self.Check and Refresh Widget Link`)
  (`/Game/Scoring/Evirement/UI/WBP_ActorStats.UpdateBars` (`self.As WBP Actor Stats`) (/ (`self.CurrentHP`) (`self.MaxHP`)) (/ (`self.CurrentStylePoints`) (`self.StylePoints`)))
  (`/Game/Scoring/Evirement/UI/WBP_ActorStats.SetTextValues` (`self.As WBP Actor Stats`) (`self.CurrentHP`) (`self.MaxHP`) (`self.CurrentStylePoints`) (`self.StylePoints`)))

(fn `Check and Refresh Widget Link`
  (`/Engine/EditorBlueprintResources/StandardMacros.IsValid` (`self.As WBP Actor Stats`)
    (:`Is Valid`
      (return))
    (:`Is Not Valid`
      (bind _aswbp_actor_stats (cast `/Game/Scoring/Evirement/UI/WBP_ActorStats` (`WidgetComponent.GetWidget` (`self.Widget`))))
      (set `self.As WBP Actor Stats` _aswbp_actor_stats)
      (return))))

(fn `DeathProcedure`
  (`self.K2_DestroyActor`))

(fn `ReceiveDamage`
  (params (InputDamage :type "Float (double-precision)"))
  (set `self.ReceivedDamage` (select `bool` (< (- (`self.CurrentHP`) InputDamage) 0.0) :`false` InputDamage :`true` (`self.CurrentHP`)))
  (set `self.ReceivedDamagePercent` (/ (`self.ReceivedDamage`) (/ (`self.MaxHP`) 100.0)))
  ;[1 1 1] Decrease HP and call death if <= 0
  (bind _output_get (set `self.CurrentHP` (- (`self.CurrentHP`) (`self.ReceivedDamage`))))
  (if (<= _output_get 0.0)
    (`self.DeathProcedure`)))

(fn `UserConstructionScript`
  (set `self.CurrentHP` (`self.MaxHP`))
  (set `self.CurrentStylePoints` (`self.StylePoints`)))