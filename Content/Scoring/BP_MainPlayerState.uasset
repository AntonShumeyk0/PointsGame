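; Player state that tracks the player's score and a style meter that drives a score multiplier.
; On BeginPlay it builds per-multiplier threshold and decay duration maps from a settings DataTable.
; IncreasePoints adds multiplied points, raises capped style points and can step the multiplier up.
; A looping one-second timer drains style at a rate derived from the current tier's span and duration, stepping the multiplier down below thresholds.
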(event `self.ReceiveBeginPlay`
  ;[1 1 1] Inititializing
  (`BlueprintMapLibrary.Map_Clear` (`self.MultiplierMaxValues`))
  (`BlueprintMapLibrary.Map_Clear` (`self.MultiplierDecreseRate`))
  (bind _outrownames (`DataTableFunctionLibrary.GetDataTableRowNames` (`self.SettingsDataTable`)))
  (for _array_element _outrownames
    (bind _returnvalue (`|GetDataTableRow` (`self.SettingsDataTable`) _array_element)
      (:`then`
        (bind (_multiplier _maxvalueformultiplier _duration) (break `/Game/Scoring/Data/ST_MultiplierSettings` _returnvalue))
        (`BlueprintMapLibrary.Map_Add` (`self.MultiplierMaxValues`) _multiplier _maxvalueformultiplier)
        (`BlueprintMapLibrary.Map_Add` (`self.MultiplierDecreseRate`) _multiplier _duration)))))

(event `self.ReceiveTick`
  (params (DeltaSeconds :type "Float (single-precision)"))
  ;[1 0.05082 0] Debug
  (if (`self.ShowDebug`)
    (`KismetSystemLibrary.PrintString` (`KismetStringLibrary.Concat_StrStr` "Current MX::  " (`KismetStringLibrary.Conv_IntToString` (`self.CurrentMultiplier`)) "  CurrentPoints:  " (`KismetStringLibrary.Conv_DoubleToString` (`self.Style Points`))) true true (struct :`G` 0.66 :`B` 1.0 :`A` 1.0) DeltaSeconds)))

(event `/Game/Scoring/BPI_PlayerState.IncreasePoints`
  (params (Points :type "Float (double-precision)") (StylePoints :type "Float (double-precision)"))
  (`self.IncreasePointsRealization` Points)
  (`self.IncreaseStylePointsRealozation` StylePoints)
  (if (not (`KismetSystemLibrary.K2_IsTimerActiveHandle` (`self.DecreaseStylePointsTimerHandle`)))
    (bind _returnvalue (`KismetSystemLibrary.K2_SetTimer` null "DecreaseStylePoints" 1.0 true))
    (set `self.DecreaseStylePointsTimerHandle` _returnvalue)))

(event `DecreaseStylePoints`
  (bind (_value _returnvalue) (`BlueprintMapLibrary.Map_Find` (`self.MultiplierMaxValues`) (- (`self.CurrentMultiplier`) 1)))
  (bind _returnvalue_2 (- (`self.Style Points`) (/ (select `bool` _returnvalue :`false` (`BlueprintMapLibrary.Map_Find` (`self.MultiplierMaxValues`) (`self.CurrentMultiplier`)) :`true` (- (`BlueprintMapLibrary.Map_Find` (`self.MultiplierMaxValues`) (`self.CurrentMultiplier`)) _value)) (`BlueprintMapLibrary.Map_Find` (`self.MultiplierDecreseRate`) (`self.CurrentMultiplier`)))))
  (bind _returnvalue_3 (< _returnvalue_2 0.0))
  ;[1 1 1] Decrease style points and multiplier check
  (if _returnvalue_3
    (`KismetSystemLibrary.K2_ClearAndInvalidateTimerHandle` (`self.DecreaseStylePointsTimerHandle`)))
  (set `self.Style Points` (select `bool` _returnvalue_3 :`false` _returnvalue_2))
  (if (and (> (`self.CurrentMultiplier`) 1) (`.ReturnValue` (`BlueprintMapLibrary.Map_Find` (`self.MultiplierMaxValues`) (- (`self.CurrentMultiplier`) 1))) (< (`self.Style Points`) (`BlueprintMapLibrary.Map_Find` (`self.MultiplierMaxValues`) (- (`self.CurrentMultiplier`) 1))))
    (`/Engine/EditorBlueprintResources/StandardMacros.DecrementInt` (`self.CurrentMultiplier`))))

(event `IncreaseStylePointsRealozation`
  (params (StylePoints :type "Float (double-precision)"))
  (bind _multipliermaxvalues (`self.MultiplierMaxValues`))
  (bind (_value _returnvalue) (`BlueprintMapLibrary.Map_Find` (`self.MultiplierMaxValues`) (`self.CurrentMultiplier`)))
  (bind _returnvalue_2 (+ StylePoints (`self.Style Points`)))
  (bind _value_2 (`BlueprintMapLibrary.Map_Find` _multipliermaxvalues (`BlueprintMapLibrary.Map_Length` _multipliermaxvalues)))
  ;[1 1 1] increase style points and multiplier
  (set `self.Style Points` (select `bool` (< _returnvalue_2 _value_2) :`false` _value_2 :`true` _returnvalue_2))
  (if (and (> (`self.Style Points`) _value) _returnvalue (`.ReturnValue` (`BlueprintMapLibrary.Map_Find` (`self.MultiplierMaxValues`) (+ (`self.CurrentMultiplier`) 1))))
    (`/Engine/EditorBlueprintResources/StandardMacros.IncrementInt` (`self.CurrentMultiplier`))))

(event `IncreasePointsRealization`
  (params (Points :type "Float (double-precision)"))
  ;[1 1 1] Points Calculations
  (set `self.Points` (+ (* Points (`self.CurrentMultiplier`)) (`self.Points`))))

(fn `UserConstructionScript`)